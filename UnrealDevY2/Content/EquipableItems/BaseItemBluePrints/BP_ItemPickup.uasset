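; BP_ItemPickup is a base item pickup actor that registers itself with the first-person character while that character is within range.
; On BeginPlay it applies its ItemMesh and WorldScale variables to the Item mesh component.
; Sphere overlap sets the character's CurrentPickup to this actor, and leaving clears it to None without checking which pickup is current.
; The pickup action itself is not handled here.
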(event OnComponentBeginOverlap(Sphere)
  (params (OverlappedComponent :type Primitive%20Component%20Object%20Reference) (OtherActor :type Actor%20Object%20Reference) (OtherComp :type Primitive%20Component%20Object%20Reference) (OtherBodyIndex :type Integer) (bFromSweep :type Boolean) (SweepResult :type Hit%20Result%20Structure%20%28by%20ref%29))
  (bind _asbp_first_person_character (Utilities|Casting|CastToBP_FirstPersonCharacter OtherActor))
  (Variables|/Game/FirstPerson/Blueprints/BP_FirstPersonCharacter.BP_FirstPersonCharacter_C|SetcurrentPickup _asbp_first_person_character self))

(event OnComponentEndOverlap(Sphere)
  (params (OverlappedComponent :type Primitive%20Component%20Object%20Reference) (OtherActor :type Actor%20Object%20Reference) (OtherComp :type Primitive%20Component%20Object%20Reference) (OtherBodyIndex :type Integer))
  (bind _asbp_first_person_character (Utilities|Casting|CastToBP_FirstPersonCharacter OtherActor))
  (Variables|/Game/FirstPerson/Blueprints/BP_FirstPersonCharacter.BP_FirstPersonCharacter_C|SetcurrentPickup _asbp_first_person_character 0))

(event EventBeginPlay
  (Components|StaticMesh|SetStaticMesh (Variables|Default|GetItem) (Variables|Default|GetItem%20Mesh))
  (Transformation|SetRelativeScale3D (Variables|Default|GetItem) (Variables|Default|GetWorldScale)))

(fn ConstructionScript)