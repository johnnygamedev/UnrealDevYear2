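; Base Blueprint for evidence items that can be tested for fingerprints, blood and gunshot residue.
; Each test function checks whether the item supports it and was already tested, then sets its tested flag on a first run.
; Results appear as messages through ShowEvidenceResult on player 0's BP_FirstPersonCharacter.
; Fingerprint and blood results follow per-item flags, while the gunshot branch is hardcoded true, so an eligible first test always finds residue.
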(event EventBeginPlay
  (|CallParentFunction) ; This node is disabled and will not be called.\nDrag off pins to build functionality.
)

(event Collision|EventActorBeginOverlap
  (params (OtherActor :type Actor%20Object%20Reference)))

(event EventTick
  (params (DeltaSeconds :type Float%20%28single-precision%29)))

(fn ConstructionScript
  (|CallParentFunction))

(fn DustforFingerprints
  (bind _returnvalue (Game|GetPlayerCharacter 0))
  (if (Variables|Default|GetCanBeDusted)
    (if (Variables|Default|GetIsDusted)
      (bind _asbp_first_person_character (Utilities|Casting|CastToBP_FirstPersonCharacter _returnvalue))
      (Default|ShowEvidenceResult _asbp_first_person_character "This item has already been dusted")
      (elif (Variables|Default|GetHasFingerprints)
        (bind _asbp_first_person_character_2 (Utilities|Casting|CastToBP_FirstPersonCharacter _returnvalue))
        (Default|ShowEvidenceResult _asbp_first_person_character_2 "Fingerprints found")
        (Variables|Default|SetIsDusted true)
        (else
          (bind _asbp_first_person_character_3 (Utilities|Casting|CastToBP_FirstPersonCharacter _returnvalue))
          (Default|ShowEvidenceResult _asbp_first_person_character_3 "This item has no fingerprints")
          (Variables|Default|SetIsDusted true))))
    (else
      (bind _asbp_first_person_character_4 (Utilities|Casting|CastToBP_FirstPersonCharacter _returnvalue))
      (Default|ShowEvidenceResult _asbp_first_person_character_4 "this item cant be dusted"))))

(fn TestforBlood
  (bind _returnvalue (Game|GetPlayerCharacter 0))
  (if (Variables|Default|GetCanBeBloodTested)
    (if (Variables|Default|GetIsBloodTested)
      (bind _asbp_first_person_character (Utilities|Casting|CastToBP_FirstPersonCharacter _returnvalue))
      (Default|ShowEvidenceResult _asbp_first_person_character "This item has already been tested for blood")
      (elif (Variables|Default|GetHasBlood)
        (bind _asbp_first_person_character_2 (Utilities|Casting|CastToBP_FirstPersonCharacter _returnvalue))
        (Default|ShowEvidenceResult _asbp_first_person_character_2 "Blood found")
        (Variables|Default|SetIsBloodTested true)
        (else
          (bind _asbp_first_person_character_3 (Utilities|Casting|CastToBP_FirstPersonCharacter _returnvalue))
          (Default|ShowEvidenceResult _asbp_first_person_character_3 "This item didnt have any blood sample")
          (Variables|Default|SetIsBloodTested true))))
    (else
      (bind _asbp_first_person_character_4 (Utilities|Casting|CastToBP_FirstPersonCharacter _returnvalue))
      (Default|ShowEvidenceResult _asbp_first_person_character_4 "This item cant be tested for blood"))))

(fn GunShotTest
  (bind _returnvalue (Game|GetPlayerCharacter 0))
  (if (Variables|Default|GetCanBeGunshotTested)
    (if (Variables|Default|GetIsGunShotTested)
      (bind _asbp_first_person_character (Utilities|Casting|CastToBP_FirstPersonCharacter _returnvalue))
      (Default|ShowEvidenceResult _asbp_first_person_character "This item has already been tested for gunshot residue")
      (elif true
        (bind _asbp_first_person_character_2 (Utilities|Casting|CastToBP_FirstPersonCharacter _returnvalue))
        (Default|ShowEvidenceResult _asbp_first_person_character_2 "Gunshot residue found")
        (Variables|Default|SetIsGunShotTested true)
        (else
          (bind _asbp_first_person_character_3 (Utilities|Casting|CastToBP_FirstPersonCharacter _returnvalue))
          (Default|ShowEvidenceResult _asbp_first_person_character_3 "No gunshot residue found")
          (Variables|Default|SetIsGunShotTested true))))
    (else
      (bind _asbp_first_person_character_4 (Utilities|Casting|CastToBP_FirstPersonCharacter _returnvalue))
      (Default|ShowEvidenceResult _asbp_first_person_character_4 "this item cant be tested for gunshot residue"))))