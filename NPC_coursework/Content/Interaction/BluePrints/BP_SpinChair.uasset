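; BP_SpinChair is an interactable chair that works as a key-gated switch for a linked door.
; Interact checks the first-person character's HasChairKey, then a timeline lerps the mesh rotation through a half turn.
; When the forward spin finishes it opens TargetDoor, while ResetState reverses the timeline to undo the spin.
; Prompt events toggle the UIAlert's visibility.
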(event EventBeginPlay)

(event Collision|EventActorBeginOverlap
  (params (OtherActor :type Actor%20Object%20Reference)))

(event EventTick
  (params (DeltaSeconds :type Float%20%28single-precision%29)))

(event EventShowInteractionPrompt
  (Development|PrintString "HIYA")
  (Rendering|SetVisibility (Variables|Default|GetUI_Alert) true false))

(event EventInteract
  (params (Instigator :type Actor%20Object%20Reference))
  (bind _asbp_first_person_character (Utilities|Casting|CastToBP_FirstPersonCharacter Instigator))
  (if (Variables|/Game/Content/FirstPerson/Blueprints/BP_FirstPersonCharacter.BP_FirstPersonCharacter_C|GetHasChairKey _asbp_first_person_character)
    (bind (_direction _rotation_alpha) (Timeline|SpinTimeline PlayFromStart)
      (:Update
        (Transformation|SetRelativeRotation (Variables|Default|GetStaticMesh) (Math|Rotator|Lerp(Rotator) "0, 0, 0" "0.000000,180.000000,0.000000" _rotation_alpha true) false false))
      (:Finished
        (if (Utilities|Enum|Equal(Enum) _direction "Forward")
          (Default|OpenDoor (Variables|Default|GetTargetDoor)))))))

(event EventResetState
  (Development|PrintString "SHOWM E" true true "(R=0.000000,G=0.660000,B=1.000000,A=1.000000)" 1e+01)
  (bind (_direction _rotation_alpha) (Timeline|SpinTimeline Reverse)
    (:Update
      (Transformation|SetRelativeRotation (Variables|Default|GetStaticMesh) (Math|Rotator|Lerp(Rotator) "0, 0, 0" "0.000000,180.000000,0.000000" _rotation_alpha true) false false))
    (:Finished
      (if (Utilities|Enum|Equal(Enum) _direction "Forward")
        (Default|OpenDoor (Variables|Default|GetTargetDoor))))))

(event EventHideIneractionPrompt
  (Rendering|SetVisibility (Variables|Default|GetUI_Alert) false false))

(fn ConstructionScript)