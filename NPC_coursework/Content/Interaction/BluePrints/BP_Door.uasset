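; BP_Door is an interactable door actor that opens by vanishing rather than animating.
; Interaction prompt events show and hide its UIAlert component, while Interact only prints a "Clue collected" debug string and does not open the door.
; OpenDoor hides the actor and disables its collision, and ResetState restores both.
; The events have no callers in this Blueprint, and showing the prompt and opening also print debug strings.
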(event Custom|OpenDoor
  (Rendering|SetActorHiddenInGame true)
  (Development|PrintString "hidden")
  (Collision|SetActorEnableCollision false))

(event EventBeginPlay)

(event Collision|EventActorBeginOverlap
  (params (OtherActor :type Actor%20Object%20Reference)))

(event EventTick
  (params (DeltaSeconds :type Float%20%28single-precision%29)))

(event EventShowInteractionPrompt
  (Development|PrintString "HIYA")
  (Rendering|SetVisibility (Variables|Default|GetUI_Alert) true false))

(event EventInteract
  (params (Instigator :type Actor%20Object%20Reference))
  (Development|PrintString "Clue collected"))

(event EventResetState
  (Rendering|SetActorHiddenInGame false)
  (Collision|SetActorEnableCollision true))

(event EventHideIneractionPrompt
  (Rendering|SetVisibility (Variables|Default|GetUI_Alert) false false))

(fn ConstructionScript)