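; BP_Drawer1 is an interactable actor, named as a drawer but built around a spin, with leftover "Chair spun" debug text in unconnected nodes.
; Prompt events toggle the UIAlert component's visibility, with a debug print on show.
; Interact plays SpinTimeline, whose alpha lerps StaticMesh's relative rotation toward a full turn.
; The lerp uses ShortestPath, which reduces the 360-degree delta to zero, so no visible spin results.
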(event EventBeginPlay)

(event Collision|EventActorBeginOverlap
  (params (OtherActor :type Actor%20Object%20Reference)))

(event EventTick
  (params (DeltaSeconds :type Float%20%28single-precision%29)))

(event EventShowInteractionPrompt
  (Development|PrintString "HIYA")
  (Rendering|SetVisibility (Variables|Default|GetUI_Alert) true false))

(event EventInteract
  (params (Instigator :type Actor%20Object%20Reference))
  (bind _rotation_alpha (Timeline|SpinTimeline Play)
    (:Update
      (Transformation|SetRelativeRotation (Variables|Default|GetStaticMesh) (Math|Rotator|Lerp(Rotator) "0, 0, 0" "0.000000,360.000000,0.000000" _rotation_alpha true) false false))))

(event EventHideIneractionPrompt
  (Rendering|SetVisibility (Variables|Default|GetUI_Alert) false false))

(fn ConstructionScript)