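; BP_ChairKey is an interactable key pickup that grants the chair key to the first-person character.
; Prompt events toggle the visibility of its UIAlert, with a debug print on show.
; Interact casts the instigator to BP_FirstPersonCharacter, sets HasChairKey, then hides the actor and disables collision instead of destroying it.
; ResetState restores visibility and collision but leaves the character's flag untouched.
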(event EventBeginPlay)

(event Collision|EventActorBeginOverlap
  (params (OtherActor :type Actor%20Object%20Reference)))

(event EventTick
  (params (DeltaSeconds :type Float%20%28single-precision%29)))

(event EventShowInteractionPrompt
  (Development|PrintString "HIYA")
  (Rendering|SetVisibility (Variables|Default|GetUI_Alert) true false))

(event EventInteract
  (params (Instigator :type Actor%20Object%20Reference))
  (bind _asbp_first_person_character (Utilities|Casting|CastToBP_FirstPersonCharacter Instigator))
  (Variables|/Game/Content/FirstPerson/Blueprints/BP_FirstPersonCharacter.BP_FirstPersonCharacter_C|SetHasChairKey _asbp_first_person_character true)
  (Rendering|SetActorHiddenInGame true)
  (Development|PrintString "hidden")
  (Collision|SetActorEnableCollision false))

(event EventResetState
  (Rendering|SetActorHiddenInGame false)
  (Collision|SetActorEnableCollision true))

(event EventHideIneractionPrompt
  (Rendering|SetVisibility (Variables|Default|GetUI_Alert) false false))

(fn ConstructionScript)