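; WanderBP is a behavior tree task that picks a random wander destination for a Workshop NPC.
; It casts the owner to WorkshopAI and its pawn to Workshop_C, and fails if that pawn is Talking.
; Otherwise it queries a navigable point within the pawn's WanderRadius, writes it to the WanderLocation blackboard key and succeeds.
; Failed casts or a failed navigation query never call FinishExecute.
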(event EventReceiveExecute
  (params (OwnerActor :type Actor%20Object%20Reference))
  (bind _asworkshop_ai (Utilities|Casting|CastToWorkshopAI OwnerActor))
  (bind _asworkshop_c (Utilities|Casting|CastToWorkshop_C (Pawn|GetControlledPawn _asworkshop_ai)))
  (if (Variables|/Game/Workshop/NPCwander/Workshop_C.Workshop_C_C|GetTalking _asworkshop_c)
    (AI|BehaviorTree|FinishExecute false)
    (else
      (bind (_randomlocation _returnvalue) (Class|NavigationSystemV1|GetRandomLocationinNavigableRadius (Transformation|GetActorLocation _asworkshop_c) (Variables|/Game/Workshop/NPCwander/Workshop_C.Workshop_C_C|GetWander%20Radius _asworkshop_c) 0 0))
      (if _returnvalue
        (AI|BehaviorTree|SetBlackboardValueasVector (Utilities|Struct|MakeBlackboardKeySelector 0 "WanderLocation" "/Script/AIModule.BlackboardKeyType_Vector") _randomlocation)
        (AI|BehaviorTree|FinishExecute true)))))